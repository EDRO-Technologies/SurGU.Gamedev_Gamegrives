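; BP_CommonEnemy is a child enemy Blueprint that defines a common enemy's max health, damage, distraction and death behavior.
; BeginPlay fills health and caches the above-head bar widget, which Tick updates with the current health percentage.
; Death runs once, stopping AI logic and playing a sword death animation before a delayed call to the parent Die.
; OnDistract briefly sets CantMove to hold the enemy in place.
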(event EventBeginPlay
  (Variables|Default|SetHealth (CallFunction|GetMaxHealth))
  (bind _asumg_above_bar (Utilities|Casting|CastToUMG_AboveBar (UserInterface|GetUserWidgetObject (Variables|Default|GetHPWidget))))
  (Variables|Default|SetHP%20bar _asumg_above_bar))

(event EventDie
  (Utilities|FlowControl|DoOnce false
    (:Completed
      (AI|Logic|StopLogic (Variables|/Script/AIModule.AIController|GetBrainComponent (AI|GetAIController self)) "")
      (Components|Animation|PlayAnimation (Variables|Character|GetMesh) "/Game/Anim/Two_Handed_Sword_Death_1_Anim.Two_Handed_Sword_Death_1_Anim" false)
      (Utilities|FlowControl|Delay 2.0)
      (|CallParentFunction))))

(event EventTick
  (params (DeltaSeconds :type Float%20%28single-precision%29))
  (|CallParentFunction DeltaSeconds)
  (Default|SetPercentage (Variables|Default|GetHP%20bar) (/ (Math|Conversions|ToFloat(Integer) (Variables|Default|GetHealth)) (Math|Conversions|ToFloat(Integer) (CallFunction|GetMaxHealth)))))

(event EventOnDistract
  (Variables|Default|SetCan't%20move true)
  (Utilities|FlowControl|Delay 0.5)
  (Variables|Default|SetCan't%20move false))

(fn ConstructionScript
  (|CallParentFunction))

(fn GetDamage
  (return (Variables|Default|GetDamage)))

(fn GetMaxHealth
  (return 150))