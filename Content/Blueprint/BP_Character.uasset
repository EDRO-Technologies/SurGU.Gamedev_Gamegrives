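; BP_Character is a character Blueprint with basic punch damage and health handling.
; Hit checks actors overlapping SweepCollision, casts each to BP_Character and calls OnPunch on any that is not itself.
; OnPunch subtracts damage from Health and prints a reaction, or calls Die when the damage would be lethal.
; Die only prints a death message and leaves Health unchanged.
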(fn ConstructionScript)

(fn OnPunch
  (params (Damage :type Integer))
  (if (<= (- (Variables|Default|GetHealth) Damage) 0)
    (CallFunction|Die)
    (else
      (Variables|Default|SetHealth (- (Variables|Default|GetHealth) Damage))
      (Development|PrintText "Ouch!"))))

(fn Die
  (Development|PrintText "Died!"))

(fn Hit
  (params (Damage :type Integer))
  (for _array_element (Collision|GetOverlappingActors (Variables|Default|GetSweepCollision) 0 :!class /Script/Engine.PrimitiveComponent)
    (bind _asbp_character (Utilities|Casting|CastToBP_Character _array_element))
    (if (not (== _asbp_character self))
      (CallFunction|OnPunch _asbp_character Damage))))