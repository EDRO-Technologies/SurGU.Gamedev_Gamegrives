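; BP_Player is the player Blueprint, which publishes its position, handles look input and ends the game on death.
; Each tick it casts the game mode to BP_TopDownGameMode and writes the actor's location into PlayerPosition.
; The IA_Look Enhanced Input action drives controller rotation, with X feeding pitch and Y feeding yaw.
; Die quits the application outright, and the construction script only calls its parent.
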(event Input|EnhancedActionEvents|EnhancedInputActionIA_Look
  (params (ActionValue :type Vector%202D%20Structure) (ElapsedSeconds :type Float%20%28double-precision%29) (TriggeredSeconds :type Float%20%28double-precision%29) (InputAction :type Input%20Action%20Object%20Reference :default "/Game/Input/Actions/IA_Look.IA_Look"))
  (:Triggered
    (Pawn|Input|AddControllerPitchInput (.x ActionValue))
    (Pawn|Input|AddControllerYawInput (.y ActionValue))))

(event EventTick
  (params (DeltaSeconds :type Float%20%28single-precision%29))
  (bind _asbp_top_down_game_mode (Utilities|Casting|CastToBP_TopDownGameMode (Game|GetGameMode)))
  (Variables|/Game/Blueprint/BP_TopDownGameMode.BP_TopDownGameMode_C|SetPlayerPosition _asbp_top_down_game_mode (.location (Transformation|GetActorTransform self))))

(fn ConstructionScript
  (|CallParentFunction))

(fn Die
  (Game|QuitGame 0 "Quit" false))